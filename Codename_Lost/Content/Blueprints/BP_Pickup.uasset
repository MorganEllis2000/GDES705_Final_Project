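; BP_Pickup is a pickup actor that highlights its mesh for interaction and saves player progress once it is collected.
; BeginPlay caches the player BP_Character and creates a dynamic outline material as the mesh overlay.
; Tick toggles that overlay from the character's shared CanInteract flag.
; Tick also watches WasPickedUp and, for codex or inventory items, uses DoOnce to save inventory, codex and position to a save slot.
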(event `self.ReceiveBeginPlay`
  (bind _asbp_character (cast `/Game/Blueprints/BP_Character` (`GameplayStatics.GetPlayerCharacter` 0)))
  (set `self.Character` _asbp_character)
  (bind _returnvalue (`PrimitiveComponent.CreateDynamicMaterialInstance` (`self.ObjectMesh`) (+ (`KismetArrayLibrary.Array_Length` (`MeshComponent.GetMaterials` (`self.ObjectMesh`))) 1) "/Game/Materials/Outline/M_Outline_Inst.M_Outline_Inst" "None"))
  (bind _output_get (set `self.NewVar_0` _returnvalue))
  (`MeshComponent.SetOverlayMaterial` (`self.ObjectMesh`) _output_get)
  (`MaterialInstanceDynamic.SetScalarParameterValue` _output_get "Outline Thickness" -1.0))

(event `self.ReceiveTick`
  (params (DeltaSeconds :type "Float (single-precision)"))
  (bind _newvar_0 (`self.NewVar_0`))
  (bind _character (`self.Character`))
  (bind _savegame (`/Game/Blueprints/BP_Character.SaveGame` _character))
  (`|ExecutionSequence`
    (:`then_0`
      (if (`CharacterController.bCanInteract` (`self.Character`))
        (`MeshComponent.SetOverlayMaterial` (`self.ObjectMesh`) _newvar_0)
        (`MaterialInstanceDynamic.SetScalarParameterValue` _newvar_0 "Outline Thickness" 3.0)
        (else
          (`MeshComponent.SetOverlayMaterial` (`self.ObjectMesh`) null))))
    (:`then_1`
      (if (`self.bWasPickedUp`)
        (if (or (`self.bCanBeAddedToCodex`) (`self.bCanBeAddedToInventory`))
          (`/Engine/EditorBlueprintResources/StandardMacros.IsValid` (`self.Character`)
            (:`Is Valid`
              (`/Engine/EditorBlueprintResources/StandardMacros.DoOnce` false
                (:`Completed`
                  (`/Game/Blueprints/BP_Character.SaveInventory` _character)
                  (`/Game/Blueprints/BP_Character.SaveCodex` _character)
                  (`/Game/Blueprints/BP_Character.SavePosition` _character)
                  (`GameplayStatics.SaveGameToSlot` _savegame "save1")
                  (`KismetSystemLibrary.PrintString` (`KismetStringLibrary.Conv_TransformToString` (`/Game/Settings/BP_Save.PlayerPos` _savegame))))))
            (:`Is Not Valid`
              (`KismetSystemLibrary.PrintString` "false"))))))))

(fn `UserConstructionScript`)