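; Player character that handles save-game persistence, damage feedback and game over.
; BeginPlay loads or creates the "save1" PlayerData, restoring inventory, codex, keys and lighter while hiding matching pickups, and loads per-level WorldData.
; Damage shows a blood overlay, plays a montage and briefly blocks zooming.
; Tick polls for death to pause on the game-over widget, saves lighter pickup and triggers a movement sound; M, P and L kill, load and save.
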(event `Key|M`
  (params (Key :type "Key Structure"))
  (:`Pressed`
    (set `HealthComponent.CurrentHealth` 0.0 (`self.Health`))))

(event `Key|P`
  (params (Key :type "Key Structure"))
  (:`Pressed`
    (bind _returnvalue (`GameplayStatics.DoesSaveGameExist` "save1"))
    (if _returnvalue
      (`self.LoadInventory`)
      (`self.LoadCodex`)
      (else
        (`KismetSystemLibrary.PrintString` "No save game")))))

(event `Key|L`
  (params (Key :type "Key Structure"))
  (:`Pressed`
    (bind _returnvalue (`GameplayStatics.DoesSaveGameExist` "save1"))
    (if _returnvalue
      (`/Engine/EditorBlueprintResources/StandardMacros.IsValid` (`self.PlayerData`)
        (:`Is Valid`
          (`self.SaveInventory`)
          (`self.SaveCodex`)
          (`GameplayStatics.SaveGameToSlot` (`self.PlayerData`) "save1"))
        (:`Is Not Valid`
          (`KismetSystemLibrary.PrintString` "invalid ")))
      (else
        (`KismetSystemLibrary.PrintString` "No save game")))))

(event `self.ReceiveAnyDamage`
  (params (Damage :type "Float (single-precision)") (DamageType :type "DamageType Object Reference") (InstigatedBy :type "Controller Object Reference") (DamageCauser :type "Actor Object Reference"))
  (bind _bloodref (`self.BloodRef`))
  (`UserWidget.AddToViewport` _bloodref 0)
  (set `self.bCanZoomIn` false)
  (`self.PlayAnimMontage` "/Game/FirstPersonArms/Character/Arms/Animations/AM_Damaged.AM_Damaged")
  (`KismetSystemLibrary.Delay` 3.0)
  (`/Game/Widgets/WBP_BloodEffect.FadeOut` _bloodref)
  (set `self.bCanZoomIn` true))

(event `self.ReceiveBeginPlay`
  (`|ExecutionSequence`
    (:`then_0`
      (bind _returnvalue (`GameplayStatics.DoesSaveGameExist` "save1"))
      (if _returnvalue
        (`self.LoadGameOnStart`)
        (`self.LoadKeys`)
        (`self.LoadLighter`)
        (else
          (`self.SaveGameOnStart`)
          (`self.SaveKeys`)
          (`GameplayStatics.SaveGameToSlot` (`self.PlayerData`) "save1"))))
    (:`then_1`
      (set `self.PostProcessComponent` (`self.PostProcess`)))
    (:`then_2`
      (bind _returnvalue_2 (`|CreateWidget` "/Game/Widgets/WBP_BloodEffect.WBP_BloodEffect_C"))
      (set `self.BloodRef` _returnvalue_2)
      (bind _returnvalue_3 (`|CreateWidget` "/Game/Widgets/WBP_GameOver.WBP_GameOver_C"))
      (set `self.WBP_GameOver` _returnvalue_3))
    (:`then_3`
      (set `self.bCanZoomIn` true))
    (:`then_4`
      (bind _returnvalue_4 (`GameplayStatics.GetCurrentLevelName` true))
      (`GameplayStatics.DoesSaveGameExist` _returnvalue_4)
      (if true
        (bind _returnvalue_5 (`GameplayStatics.GetCurrentLevelName` true))
        (bind _returnvalue_6 (`GameplayStatics.LoadGameFromSlot` _returnvalue_5))
        (bind _asbp_world_data (cast `/Game/Settings/BP_WorldData` _returnvalue_6))
        (set `self.WorldData` _asbp_world_data)))))

(event `self.ReceiveTick`
  (params (DeltaSeconds :type "Float (single-precision)"))
  (`|ExecutionSequence`
    (:`then_0`
      (if (<= (`HealthComponent.CurrentHealth` (`self.Health`)) 0.0)
        (`/Engine/EditorBlueprintResources/StandardMacros.DoOnce` false
          (:`Completed`
            (`UserWidget.AddToViewport` (`self.WBP_GameOver`) 0)
            (`KismetSystemLibrary.Delay` 2.0)
            (`GameplayStatics.SetGamePaused` true)
            (`WidgetBlueprintLibrary.SetInputMode_UIOnlyEx` (`GameplayStatics.GetPlayerController` 0) null)
            (set `PlayerController.bShowMouseCursor` true (`GameplayStatics.GetPlayerController` 0))))))
    (:`then_1`
      (bind _asgm_codename_lost (cast `/Game/Settings/GM_CodenameLost` (`GameplayStatics.GetGameMode`)))
      (if (`Codename_LostGameModeBase.bHasLighter` _asgm_codename_lost)
        (`/Engine/EditorBlueprintResources/StandardMacros.DoOnce` false
          (:`Completed`
            (set `/Game/Settings/BP_PlayerData.PickedUpLighter` true (`self.PlayerData`))
            (`GameplayStatics.SaveGameToSlot` (`self.PlayerData`) "save1")))))
    (:`then_2`
      (if (>= (`KismetMathLibrary.VSize` (`self.GetVelocity`)) 50.0)
        (`/Engine/EditorBlueprintResources/StandardMacros.DoOnce` false :!label _label
          (:`Completed`
            (`GameplayStatics.PlaySoundAtLocation` (`self.Sound`) (`self.K2_GetActorLocation`) (struct) 1.0 1.0 0.0 null null null null)))
        (else
          (goto _label :!via `Reset`))))))

(fn `CheckHealth`
  (returns (NewParam :type Boolean))
  (return (<= (`HealthComponent.CurrentHealth` (`self.Health`)) 0.0)))

(fn `LoadCodex`
  (for _array_element (`/Game/Settings/BP_PlayerData.CodexArray` (`self.PlayerData`))
    (`self.AddToCodex` _array_element)))

(fn `LoadGameOnStart`
  (bind _returnvalue (`GameplayStatics.LoadGameFromSlot` "save1"))
  (bind _asbp_player_data (cast `/Game/Settings/BP_PlayerData` _returnvalue))
  (set `self.PlayerData` _asbp_player_data)
  (for _array_element (`/Game/Settings/BP_PlayerData.InventoryArray` (`self.PlayerData`))
    (`/Engine/EditorBlueprintResources/StandardMacros.IsValid` _array_element
      (:`Is Valid`
        (`self.AddToInventory` _array_element)
        (bind _outactors (`GameplayStatics.GetAllActorsOfClass` "/Script/Codename_Lost.Pickup"))
        (for _array_element_2 _outactors
          (`/Engine/EditorBlueprintResources/StandardMacros.IsValid` _array_element_2
            (:`Is Valid`
              (for _array_element_3 (`self._inventory`)
                (`/Engine/EditorBlueprintResources/StandardMacros.IsValid` _array_element_3
                  (:`Is Valid`
                    (if (`KismetTextLibrary.EqualEqual_TextText` (`Pickup.ObjectName` _array_element_3) (`Pickup.ObjectName` _array_element_2))
                      (`Pickup.Show` _array_element_3 false)
                      (for _array_element_4 (`/Game/Settings/BP_PlayerData.CodexArray` (`self.PlayerData`))
                        (`self.AddToCodex` _array_element_4)
                        (bind _outactors_2 (`GameplayStatics.GetAllActorsOfClass` "/Script/Codename_Lost.Pickup"))
                        (for _array_element_5 _outactors_2
                          (`/Engine/EditorBlueprintResources/StandardMacros.IsValid` _array_element_5
                            (:`Is Valid`
                              (for _array_element_6 (`self._Codex`)
                                (`/Engine/EditorBlueprintResources/StandardMacros.IsValid` _array_element_6
                                  (:`Is Valid`
                                    (if (`KismetTextLibrary.EqualEqual_TextText` (`Pickup.ObjectName` _array_element_6) (`Pickup.ObjectName` _array_element_5))
                                      (`Pickup.Show` _array_element_6 false))))))))))))))))))))

(fn `LoadInventory`
  (for _array_element (`/Game/Settings/BP_PlayerData.InventoryArray` (`self.PlayerData`))
    (`self.AddToInventory` _array_element)))

(fn `LoadKeys`
  (bind _asgm_codename_lost (cast `/Game/Settings/GM_CodenameLost` (`GameplayStatics.GetGameMode`)))
  (set `Codename_LostGameModeBase.TMapOfKeys` (`/Game/Settings/BP_PlayerData.PickedUpKeys` (`self.PlayerData`)) _asgm_codename_lost))

(fn `LoadLighter`
  (bind _asgm_codename_lost (cast `/Game/Settings/GM_CodenameLost` (`GameplayStatics.GetGameMode`)))
  (set `Codename_LostGameModeBase.bHasLighter` (`/Game/Settings/BP_PlayerData.PickedUpLighter` (`self.PlayerData`)) _asgm_codename_lost))

(fn `LoadPosition`
  (bind _playerpos (`/Game/Settings/BP_PlayerData.PlayerPos` (`self.PlayerData`)))
  (`self.K2_SetActorTransform` _playerpos)
  (`KismetSystemLibrary.PrintString` (`KismetStringLibrary.Conv_TransformToString` _playerpos)))

(fn `SaveCodex`
  (for (_array_element _array_index) (`self._Codex`)
    (`KismetArrayLibrary.Array_Set` (`/Game/Settings/BP_PlayerData.CodexArray` (`self.PlayerData`)) _array_index _array_element)))

(fn `SaveGameOnStart`
  (bind _playerdata (`self.PlayerData`))
  (bind _playerdata_2 (`self.PlayerData`))
  (bind _returnvalue (`GameplayStatics.CreateSaveGameObject` "/Game/Settings/BP_PlayerData.BP_PlayerData_C"))
  (set `self.PlayerData` _returnvalue)
  (set `/Game/Settings/BP_PlayerData.InventoryArray` (`|MakeArray` (`/Game/Settings/BP_PlayerData.InventoryItem1` _playerdata_2) (`/Game/Settings/BP_PlayerData.InventoryItem2` _playerdata_2) (`/Game/Settings/BP_PlayerData.InventoryItem3` _playerdata_2) (`/Game/Settings/BP_PlayerData.InventoryItem4` _playerdata_2) (`/Game/Settings/BP_PlayerData.InventoryItem5` _playerdata_2) (`/Game/Settings/BP_PlayerData.InventoryItem6` _playerdata_2) (`/Game/Settings/BP_PlayerData.InventoryItem7` _playerdata_2) (`/Game/Settings/BP_PlayerData.InventoryItem8` _playerdata_2)) (`self.PlayerData`))
  (set `/Game/Settings/BP_PlayerData.CodexArray` (`|MakeArray` (`/Game/Settings/BP_PlayerData.CodexItem1` _playerdata) (`/Game/Settings/BP_PlayerData.CodexItem2` _playerdata) (`/Game/Settings/BP_PlayerData.CodexItem3` _playerdata) (`/Game/Settings/BP_PlayerData.CodexItem4` _playerdata) (`/Game/Settings/BP_PlayerData.CodexItem5` _playerdata) (`/Game/Settings/BP_PlayerData.CodexItem6` _playerdata) (`/Game/Settings/BP_PlayerData.CodexItem7` _playerdata) (`/Game/Settings/BP_PlayerData.CodexItem8` _playerdata)) (`self.PlayerData`))
  (`GameplayStatics.SaveGameToSlot` (`self.PlayerData`) "save1"))

(fn `SaveInventory`
  (for (_array_element _array_index) (`self._inventory`)
    (`KismetArrayLibrary.Array_Set` (`/Game/Settings/BP_PlayerData.InventoryArray` (`self.PlayerData`)) _array_index _array_element)))

(fn `SaveKeys`
  (bind _asgm_codename_lost (cast `/Game/Settings/GM_CodenameLost` (`GameplayStatics.GetGameMode`)))
  (set `/Game/Settings/BP_PlayerData.PickedUpKeys` (`Codename_LostGameModeBase.TMapOfKeys` _asgm_codename_lost) (`self.PlayerData`)))

(fn `SaveLighter`)

(fn `SavePosition`
  (set `/Game/Settings/BP_WorldData.PlayerPos` (`self.GetTransform`) (`self.WorldData`)))

(fn `UserConstructionScript`)