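; Shadow puzzle actor that briefly freezes the player's camera look when the puzzle is engaged or solved.
; It caches the player character as CharacterController on BeginPlay, then polls its InteractingWithShadowPuzzle flag and its own IsSolved flag on Tick.
; Each flag fires a one-shot two-second look-input lock through DoOnce gates that are never reset.
; While the player is not interacting, look input is reset every tick, which also clears the solved lock.
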(event `self.ReceiveBeginPlay`
  (bind _ascharacter_controller (cast `CharacterController` (`GameplayStatics.GetPlayerCharacter` 0)))
  (set `self.CharacterController` _ascharacter_controller))

(event `self.ReceiveTick`
  (params (DeltaSeconds :type "Float (single-precision)"))
  (bind _returnvalue (`GameplayStatics.GetPlayerController` 0))
  (bind _returnvalue_2 (`GameplayStatics.GetPlayerController` 0))
  (`|ExecutionSequence`
    (:`then_0`
      (if (`CharacterController.bInteractingWithShadowPuzzle` (`self.CharacterController`))
        (`/Engine/EditorBlueprintResources/StandardMacros.DoOnce` false
          (:`Completed`
            (`Controller.SetIgnoreLookInput` _returnvalue_2 true)
            (`KismetSystemLibrary.Delay` 2.0)
            (`Controller.ResetIgnoreLookInput` _returnvalue_2)))
        (else
          (`Controller.ResetIgnoreLookInput` _returnvalue_2))))
    (:`then_1`
      (if (`self.bIsSolved`)
        (`/Engine/EditorBlueprintResources/StandardMacros.DoOnce` false
          (:`Completed`
            (`Controller.SetIgnoreLookInput` _returnvalue true)
            (`KismetSystemLibrary.Delay` 2.0)
            (`Controller.ResetIgnoreLookInput` _returnvalue)))))))

(fn `UserConstructionScript`)