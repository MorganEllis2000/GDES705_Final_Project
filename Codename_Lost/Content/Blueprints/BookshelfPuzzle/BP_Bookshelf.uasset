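; BP_Bookshelf tracks whether a bookshelf puzzle is solved and persists that state per level.
; Three seconds after BeginPlay, it loads any BP_WorldData save in the slot named after the current level and restores IsBookshelfOpen.
; Tick polls that flag and, through a DoOnce, writes it back to the save when open.
; Nothing here opens the shelf; the post-load open check is empty.
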(event `self.ReceiveBeginPlay`
  (`KismetSystemLibrary.Delay` 3.0)
  (bind _returnvalue (`GameplayStatics.GetCurrentLevelName` true))
  (bind _returnvalue_2 (`GameplayStatics.DoesSaveGameExist` _returnvalue))
  (if _returnvalue_2
    (bind _returnvalue_3 (`GameplayStatics.GetCurrentLevelName` true))
    (bind _returnvalue_4 (`GameplayStatics.LoadGameFromSlot` _returnvalue_3))
    (bind _asbp_world_data (cast `/Game/Settings/BP_WorldData` _returnvalue_4))
    (set `self.WorldData` _asbp_world_data)
    (`self.LoadPuzzleState`)
    (if (`self.bIsBookshelfOpen`)
      _)))

(event `self.ReceiveTick`
  (params (DeltaSeconds :type "Float (single-precision)"))
  (if (`self.bIsBookshelfOpen`)
    (`/Engine/EditorBlueprintResources/StandardMacros.DoOnce` false
      (:`Completed`
        (`self.SavePuzzleState`)
        (bind _returnvalue (`GameplayStatics.GetCurrentLevelName` true))
        (`GameplayStatics.SaveGameToSlot` (`self.WorldData`) _returnvalue)))))

(fn `LoadPuzzleState`
  (set `self.bIsBookshelfOpen` (`/Game/Settings/BP_WorldData.BookshelfPuzzleSolved` (`self.WorldData`))))

(fn `SavePuzzleState`
  (set `/Game/Settings/BP_WorldData.BookshelfPuzzleSolved` (`self.bIsBookshelfOpen`) (`self.WorldData`)))

(fn `UserConstructionScript`)