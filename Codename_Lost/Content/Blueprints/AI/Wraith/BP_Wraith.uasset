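; Wraith AI Blueprint that destroys itself once its Health component's current health reaches zero, checked every Tick.
; BeginPlay and MoveToRandomLocation are empty, and the random navmesh roaming logic sits in disconnected nodes.
; A sprint cooldown built on DoOnce and walk speed changes is also left over, with its chase move and delay never executed.
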(event `self.ReceiveTick`
  (params (DeltaSeconds :type "Float (single-precision)"))
  (if (<= (`HealthComponent.CurrentHealth` (`self.Health`)) 0.0)
    (`self.K2_DestroyActor` self)))

(event `self.ReceiveBeginPlay`)

(event `MoveToRandomLocation`)

(event `CanSprintAgain`
  (`/Engine/EditorBlueprintResources/StandardMacros.DoOnce` false :!via `Reset`
    (:`Completed`
      (set `CharacterMovementComponent.MaxWalkSpeed` 150.0 (`self.CharacterMovement`)))))

(fn `UserConstructionScript`)