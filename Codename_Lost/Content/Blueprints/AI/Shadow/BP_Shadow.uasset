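; BP_Shadow is a Shadow AI enemy that attacks with a damage sphere and stays dead across level loads.
; Tick syncs attack state with the blackboard and resizes the sphere after a delay, while damage events set a blackboard flag.
; At zero health it records itself in the level-named save, then destroys itself, and saved kills are removed on BeginPlay.
; ChangeVignette derives post-process vignette from player distance, though nothing here calls it.
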(event `self.ReceiveBeginPlay`
  (`KismetSystemLibrary.Delay` 0.2)
  (`self.Save/Load`)
  (bind _ascharacter_controller (cast `CharacterController` (`GameplayStatics.GetPlayerCharacter` 0)))
  (set `self.Player` _ascharacter_controller))

(event `self.ReceiveTick`
  (params (DeltaSeconds :type "Float (single-precision)"))
  (`|ExecutionSequence`
    (:`then_0`
      (if (not (`self.IsDying`))
        (set `self.keyName` "IsAttacking")
        (set `self.IsAttacking` (`BlackboardComponent.GetValueAsBool` (`AIBlueprintHelperLibrary.GetBlackboard` self) (`self.keyName`)))
        (bind _output_get (set `self.keyName` "CanAttack"))
        (`BlackboardComponent.SetValueAsBool` (`AIBlueprintHelperLibrary.GetBlackboard` self) _output_get (`self.CanAttack`))
        (if (`self.IsAttacking`)
          (`KismetSystemLibrary.Delay` 1.0)
          (`SphereComponent.SetSphereRadius` (`self.DamageSphere`) 32.0 true))))
    (:`then_1`
      (if (<= (`HealthComponent.CurrentHealth` (`self.Health`)) 0.0)
        (`/Engine/EditorBlueprintResources/StandardMacros.DoOnce` false
          (:`Completed`
            (set `CharacterMovementComponent.MaxWalkSpeed` 0.0 (`self.CharacterMovement`))
            (`BlackboardComponent.SetValueAsBool` (`AIBlueprintHelperLibrary.GetBlackboard` self) (`self.IsDead`) true)
            (set `self.IsDying` true)
            (`self.SetWasKilled`)
            (bind _returnvalue (`GameplayStatics.GetCurrentLevelName` true))
            (`GameplayStatics.SaveGameToSlot` (`self.WorldData`) _returnvalue)
            (`self.DetachFromControllerPendingDestroy` self)
            (`KismetSystemLibrary.Delay` 3.4)
            (`self.K2_DestroyActor`)))))))

(event `self.ReceiveAnyDamage`
  (params (Damage :type "Float (single-precision)") (DamageType :type "DamageType Object Reference") (InstigatedBy :type "Controller Object Reference") (DamageCauser :type "Actor Object Reference"))
  (bind _output_get (set `self.keyName` "WasDamaged"))
  (`BlackboardComponent.SetValueAsBool` (`AIBlueprintHelperLibrary.GetBlackboard` (`AIBlueprintHelperLibrary.GetAIController` self)) _output_get true))

(fn `ChangeVignette`
  (bind _returnvalue (`BlackboardComponent.GetValueAsFloat` (`AIBlueprintHelperLibrary.GetBlackboard` (`AIBlueprintHelperLibrary.GetAIController` self)) (stale _output_get)))
  (if (> _returnvalue 600.0)
    (set `PostProcessComponent.Settings` (make `PostProcessSettings` :`VignetteIntensity` 1.0) (`self.PostProcess`))
    (else
      (bind _output_get (set `self.keyName` "DistFromPlayer"))
      (bind _returnvalue_2 (`KismetMathLibrary.Lerp` (- 3.0 (`KismetMathLibrary.NormalizeToRange` _returnvalue 1.0 300.0)) (`self.OldVignetteValue`)))
      (set `self.OldVignetteValue` _returnvalue_2)
      (set `PostProcessComponent.Settings` (make `PostProcessSettings` :`VignetteIntensity` _returnvalue_2) (`self.PostProcess`)))))

(fn `Save/Load`
  (bind _returnvalue (`GameplayStatics.GetCurrentLevelName` true))
  (bind _returnvalue_2 (`GameplayStatics.DoesSaveGameExist` _returnvalue))
  (if _returnvalue_2
    (bind _returnvalue_3 (`GameplayStatics.GetCurrentLevelName` true))
    (bind _returnvalue_4 (`GameplayStatics.LoadGameFromSlot` _returnvalue_3))
    (bind _asbp_world_data (cast `/Game/Settings/BP_WorldData` _returnvalue_4))
    (bind _output_get (set `self.WorldData` _asbp_world_data))
    (if (`BlueprintMapLibrary.Map_Contains` (`/Game/Settings/BP_WorldData.MapOfEnemies` _output_get) (`KismetSystemLibrary.GetObjectName` self))
      (`self.K2_DestroyActor`))))

(fn `SetWasKilled`
  (`BlueprintMapLibrary.Map_Add` (`/Game/Settings/BP_WorldData.MapOfEnemies` (`self.WorldData`)) (`KismetSystemLibrary.GetObjectName` self)))

(fn `UserConstructionScript`)