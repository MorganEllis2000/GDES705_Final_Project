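; Four-tumbler padlock puzzle that opens a linked Unlockable when the dialed digits match its Combination.
; While the character interacts, player input is suspended, A/D select a BP_Tumbler child actor, W/S spin it and F exits.
; Tick polls the combination; on success the lock drops with physics, unlocks and destroys itself.
; Solved state saves to BP_WorldData in a per-level slot, so BeginPlay removes already solved locks.
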(event `self.ReceiveBeginPlay`
  (bind _ascharacter_controller (cast `CharacterController` (`GameplayStatics.GetPlayerCharacter` 0)))
  (set `self.Character` _ascharacter_controller)
  (bind _output_get (set `self.TumblerArray` (`|MakeArray` (cast `/Game/Blueprints/PadlockPuzzle/BP_Tumbler` (`ChildActorComponent.ChildActor` (`self.LockTumblerOne`)) :!pure true) (cast `/Game/Blueprints/PadlockPuzzle/BP_Tumbler` (`ChildActorComponent.ChildActor` (`self.LockTumblerTwo`)) :!pure true) (cast `/Game/Blueprints/PadlockPuzzle/BP_Tumbler` (`ChildActorComponent.ChildActor` (`self.LockTumblerThree`)) :!pure true) (cast `/Game/Blueprints/PadlockPuzzle/BP_Tumbler` (`ChildActorComponent.ChildActor` (`self.LockTumblerFour`)) :!pure true))))
  (set `self.CurrentSelectedTumbler` (`|GetArrayItem` _output_get))
  (set `self.CurrentSelectedTumblerValue` 0)
  (`SceneComponent.SetVisibility` (`self.CurrentSelectionUI`) false false)
  (`KismetSystemLibrary.Delay` 3.0)
  (bind _returnvalue (`GameplayStatics.GetCurrentLevelName` true))
  (bind _returnvalue_2 (`GameplayStatics.DoesSaveGameExist` _returnvalue))
  (if _returnvalue_2
    (bind _returnvalue_3 (`GameplayStatics.GetCurrentLevelName` true))
    (bind _returnvalue_4 (`GameplayStatics.LoadGameFromSlot` _returnvalue_3))
    (bind _asbp_world_data (cast `/Game/Settings/BP_WorldData` _returnvalue_4))
    (set `self.WorldData` _asbp_world_data)
    (`self.LoadPadlockState`)
    (if (`self.IsSolved`)
      (`SceneComponent.SetVisibility` (`self.SkeletalMesh`) false true)
      (`PrimitiveComponent.SetCollisionEnabled` (`self.SkeletalMesh`) "NoCollision")
      (`/Game/Blueprints/PadlockPuzzle/BP_Unlockable.Unlock` (`self.Unlockable`))
      (`self.K2_DestroyActor`))))

(event `self.ReceiveTick`
  (params (DeltaSeconds :type "Float (single-precision)"))
  (bind _returnvalue (`GameplayStatics.GetPlayerController` 0))
  (bind _returnvalue_2 (`GameplayStatics.GetPlayerController` 0))
  (`|ExecutionSequence`
    (:`then_0`
      (`KismetSystemLibrary.Delay` 1.0)
      (bind _combomatch_ (`self.CheckCombination`))
      (if _combomatch_
        (set `self.IsSolved` _combomatch_)
        (`/Engine/EditorBlueprintResources/StandardMacros.DoOnce` false
          (:`Completed`
            (set `self.LockedState` true)
            (`KismetSystemLibrary.Delay` 1.0)
            (set `self.LockedState` false)
            (`SkeletalMeshComponent.SetAllBodiesSimulatePhysics` (`self.SkeletalMesh`) true)
            (`KismetSystemLibrary.Delay` 0.4)
            (`/Game/Blueprints/PadlockPuzzle/BP_Unlockable.Unlock` (`self.Unlockable`))
            (`KismetSystemLibrary.Delay` 2.0)
            (`SkeletalMeshComponent.SetAllBodiesSimulatePhysics` (`self.SkeletalMesh`) false)
            (`PrimitiveComponent.SetCollisionEnabled` (`self.Box`) "NoCollision")
            (`self.K2_DestroyActor`)))))
    (:`then_1`
      (if (`self.IsSolved`)
        (set `CharacterController.bInteractingWithPadlockPuzzle` false (`self.Character`))
        (`self.SavePadlockState`)
        (bind _returnvalue_3 (`GameplayStatics.GetCurrentLevelName` true))
        (`GameplayStatics.SaveGameToSlot` (`self.WorldData`) _returnvalue_3)))
    (:`then_2`
      (if (`CharacterController.bInteractingWithPadlockPuzzle` (`self.Character`))
        (`/Engine/EditorBlueprintResources/StandardMacros.DoOnce` false
          (:`Completed`
            (`Controller.SetIgnoreLookInput` _returnvalue true)
            (`self.DisableInput` (`GameplayStatics.GetPlayerCharacter` 0) _returnvalue)
            (set `self.InPadlockPuzzle` true)
            (`KismetSystemLibrary.Delay` 1.5)
            (`SceneComponent.SetVisibility` (`self.CurrentSelectionUI`) true false)))
        (elif (`self.InPadlockPuzzle`)
          (`KismetSystemLibrary.Delay` 2.0)
          (`Controller.ResetIgnoreLookInput` _returnvalue_2)
          (`self.EnableInput` (`GameplayStatics.GetPlayerCharacter` 0) _returnvalue_2)
          (set `self.InPadlockPuzzle` false)
          (`SceneComponent.SetVisibility` (`self.CurrentSelectionUI`) false false))))))

(event `Key|F`
  (params (Key :type "Key Structure"))
  (:`Pressed`
    (if (`CharacterController.bInteractingWithPadlockPuzzle` (`self.Character`))
      (set `CharacterController.bInteractingWithPadlockPuzzle` false (`self.Character`)))))

(event `Key|D`
  (params (Key :type "Key Structure"))
  (bind _tumblerarray (`self.TumblerArray`))
  (bind (_relativelocation_x _relativelocation_y _relativelocation_z) (`KismetMathLibrary.BreakVector` (`SceneComponent.RelativeLocation` (`self.CurrentSelectionUI`))))
  ;[0.01153 0.03975 0.1302] Change the currently selected tumbler
  (:`Pressed`
    (if (`CharacterController.bInteractingWithPadlockPuzzle` (`self.Character`))
      (if (< (`self.CurrentSelectedTumblerValue`) 3)
        (bind _output_get (set `self.CurrentSelectedTumblerValue` (+ (`self.CurrentSelectedTumblerValue`) 1)))
        (set `self.CurrentSelectedTumbler` (`|GetArrayItem` _tumblerarray _output_get))
        (`SceneComponent.K2_SetRelativeLocation` (`self.CurrentSelectionUI`) (`KismetMathLibrary.MakeVector` (+ _relativelocation_x 5.0) _relativelocation_y _relativelocation_z) false false)
        (else
          (bind _output_get_2 (set `self.CurrentSelectedTumblerValue` 0))
          (set `self.CurrentSelectedTumbler` (`|GetArrayItem` _tumblerarray _output_get_2))
          (`SceneComponent.K2_SetRelativeLocation` (`self.CurrentSelectionUI`) (1.0 0.0 15.0) false false))))))

(event `Key|A`
  (params (Key :type "Key Structure"))
  (bind _tumblerarray (`self.TumblerArray`))
  (bind (_relativelocation_x _relativelocation_y _relativelocation_z) (`KismetMathLibrary.BreakVector` (`SceneComponent.RelativeLocation` (`self.CurrentSelectionUI`))))
  ;[0.01153 0.03975 0.1302] Change the currently selected tumbler
  (:`Pressed`
    (if (`CharacterController.bInteractingWithPadlockPuzzle` (`self.Character`))
      (if (!= (`self.CurrentSelectedTumblerValue`) 0)
        (bind _output_get (set `self.CurrentSelectedTumblerValue` (- (`self.CurrentSelectedTumblerValue`) 1)))
        (set `self.CurrentSelectedTumbler` (`|GetArrayItem` _tumblerarray _output_get))
        (`SceneComponent.K2_SetRelativeLocation` (`self.CurrentSelectionUI`) (`KismetMathLibrary.MakeVector` (- _relativelocation_x 5.0) _relativelocation_y _relativelocation_z) false false)
        (else
          (bind _output_get_2 (set `self.CurrentSelectedTumblerValue` 3))
          (set `self.CurrentSelectedTumbler` (`|GetArrayItem` _tumblerarray _output_get_2))
          (`SceneComponent.K2_SetRelativeLocation` (`self.CurrentSelectionUI`) (16.0 0.0 15.0) false false))))))

(event `Key|W`
  (params (Key :type "Key Structure"))
  ;[0 0.04954 0.2083] Spin the tumblers
  (:`Pressed`
    (if (`CharacterController.bInteractingWithPadlockPuzzle` (`self.Character`))
      (`/Game/Blueprints/PadlockPuzzle/BP_Tumbler.SpinTumbler` (`self.CurrentSelectedTumbler`)))))

(event `Key|S`
  (params (Key :type "Key Structure"))
  ;[0 0.04954 0.2083] Spin the tumblers
  (:`Pressed`
    (if (`CharacterController.bInteractingWithPadlockPuzzle` (`self.Character`))
      (`/Game/Blueprints/PadlockPuzzle/BP_Tumbler.SpinTumblerAnti` (`self.CurrentSelectedTumbler`)))))

(fn `CheckCombination`
  (returns (`ComboMatch?` :type Boolean))
  (return (`KismetStringLibrary.EqualEqual_StrStr` (`self.Combination`) (`KismetStringLibrary.Concat_StrStr` (`KismetStringLibrary.Conv_IntToString` (`/Game/Blueprints/PadlockPuzzle/BP_Tumbler.TumblerNumber` (cast `/Game/Blueprints/PadlockPuzzle/BP_Tumbler` (`ChildActorComponent.ChildActor` (`self.LockTumblerOne`)) :!pure true))) (`KismetStringLibrary.Conv_IntToString` (`/Game/Blueprints/PadlockPuzzle/BP_Tumbler.TumblerNumber` (cast `/Game/Blueprints/PadlockPuzzle/BP_Tumbler` (`ChildActorComponent.ChildActor` (`self.LockTumblerTwo`)) :!pure true))) (`KismetStringLibrary.Conv_IntToString` (`/Game/Blueprints/PadlockPuzzle/BP_Tumbler.TumblerNumber` (cast `/Game/Blueprints/PadlockPuzzle/BP_Tumbler` (`ChildActorComponent.ChildActor` (`self.LockTumblerThree`)) :!pure true))) (`KismetStringLibrary.Conv_IntToString` (`/Game/Blueprints/PadlockPuzzle/BP_Tumbler.TumblerNumber` (cast `/Game/Blueprints/PadlockPuzzle/BP_Tumbler` (`ChildActorComponent.ChildActor` (`self.LockTumblerFour`)) :!pure true)))))))

(fn `LoadPadlockState`
  (set `self.IsSolved` (`/Game/Settings/BP_WorldData.PadlockPuzzleSolved` (`self.WorldData`))))

(fn `SavePadlockState`
  (set `/Game/Settings/BP_WorldData.PadlockPuzzleSolved` (`self.IsSolved`) (`self.WorldData`)))

(fn `UserConstructionScript`)