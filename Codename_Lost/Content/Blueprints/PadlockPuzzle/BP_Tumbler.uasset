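; BP_Tumbler is a single numbered padlock puzzle tumbler that starts on a random digit from 0 to 9.
; SpinTumbler and SpinTumblerAnti roll the mesh forward or backward via timelines, each gated by a DoOnce and a shared IsSpinning cooldown set after rotation.
; When a spin finishes, it plays a directional sound and NumberCheck derives TumblerNumber from the accumulated roll, which goes negative when wound backward past zero.
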(event `self.ReceiveBeginPlay`
  (`self.RandomiseTumbler`))

(event `SpinTumbler`
  (if (not (`self.IsSpinning`))
    (`/Engine/EditorBlueprintResources/StandardMacros.DoOnce` false :!label _label
      (:`Completed`
        (bind (_direction _newtrack_1) (`Timeline|RotateTumblr` :!via `PlayFromStart`)
          (:`Update`
            (bind _returnvalue (+ (`self.TumblerRotation`) _newtrack_1))
            (`SceneComponent.K2_SetRelativeRotation` (`self.TumblerMesh`) (`KismetMathLibrary.MakeRotator` _returnvalue) false false))
          (:`Finished`
            (set `self.TumblerRotation` _returnvalue)
            (`self.NumberCheck`)
            (set `self.IsSpinning` true)
            (`GameplayStatics.PlaySoundAtLocation` "/Game/Audio/Padlock/SW_PadlockForward.SW_PadlockForward" (`self.K2_GetActorLocation`) (struct) 1.0 1.0 0.0 null null null null)
            (`KismetSystemLibrary.Delay` 0.2)
            (set `self.IsSpinning` false)
            (`self.ResetTumbler`)
            (if (>= (`self.TumblerRotation`) 360.0)
              (set `self.TumblerRotation` 0.0))))))))

(event `ResetTumbler`
  (goto _label :!via `Reset`))

(event `SpinTumblerAnti`
  (if (not (`self.IsSpinning`))
    (`/Engine/EditorBlueprintResources/StandardMacros.DoOnce` false :!label _label_2
      (:`Completed`
        (bind (_direction _newtrack_1) (`Timeline|Timeline` :!via `PlayFromStart`)
          (:`Update`
            (bind _returnvalue (- (`self.TumblerRotation`) _newtrack_1))
            (`SceneComponent.K2_SetRelativeRotation` (`self.TumblerMesh`) (`KismetMathLibrary.MakeRotator` _returnvalue) false false))
          (:`Finished`
            (set `self.TumblerRotation` _returnvalue)
            (`self.NumberCheck`)
            (set `self.IsSpinning` true)
            (`GameplayStatics.PlaySoundAtLocation` "/Game/Audio/Padlock/SW_PadlockBackward.SW_PadlockBackward" (`self.K2_GetActorLocation`) (struct) 1.0 1.0 0.0 null null null null)
            (`KismetSystemLibrary.Delay` 0.2)
            (set `self.IsSpinning` false)
            (`self.ResetTumblerAnti`)
            (if (<= (`self.TumblerRotation`) -360.0)
              (set `self.TumblerRotation` 0.0))))))))

(event `ResetTumblerAnti`
  (goto _label_2 :!via `Reset`))

(fn `NumberCheck`
  (if (== (`KismetMathLibrary.FTrunc` (`self.TumblerRotation`)) 0)
    (set `self.TumblerNumber` 0)
    (else
      (set `self.TumblerNumber` (/ (`KismetMathLibrary.FTrunc` (`self.TumblerRotation`)) 36)))))

(fn `RandomiseTumbler`
  (bind _output_get (set `self.TumblerNumber` (`KismetMathLibrary.RandomIntegerInRange` 0 9)))
  (bind _output_get_2 (set `self.TumblerRotation` (`KismetMathLibrary.Conv_IntToDouble` (* _output_get 36))))
  (`SceneComponent.K2_SetRelativeRotation` (`self.TumblerMesh`) (`KismetMathLibrary.MakeRotator` _output_get_2) false false)
  (`self.NumberCheck`))

(fn `UserConstructionScript`)