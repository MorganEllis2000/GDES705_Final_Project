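; BP_Cobweb is a cobweb obstacle that burns away when overlapped while the game mode reports the player has a lighter.
; On BeginPlay it creates a dynamic instance of a dissolve-area material and caches GM_CodenameLost.
; An overlap with the lighter starts the dissolve, otherwise it prints a debug warning.
; Tick then raises the material's Bounds Scale at a frame-rate-dependent rate and destroys the actor at the limit.
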(event `self.ReceiveBeginPlay`
  (bind _returnvalue (`PrimitiveComponent.CreateDynamicMaterialInstance` (`self.StaticMeshComponent`) 0 "/Game/Materials/DissolveArea/M_DissolveArea_Inst.M_DissolveArea_Inst" "None"))
  (set `self.DynamicMaterial` _returnvalue)
  (bind _asgm_codename_lost (cast `/Game/Settings/GM_CodenameLost` (`GameplayStatics.GetGameMode`)))
  (set `self.GameMode` _asgm_codename_lost))

(event `self.ReceiveActorBeginOverlap`
  (params (OtherActor :type "Actor Object Reference"))
  (if (`Codename_LostGameModeBase.bHasLighter` (`self.GameMode`))
    (set `self.StartDissolve` true)
    (else
      (`KismetSystemLibrary.PrintString` "NEED LIGHTER"))))

(event `self.ReceiveTick`
  (params (DeltaSeconds :type "Float (single-precision)"))
  (if (`self.StartDissolve`)
    (if (< (`self.Bounds Scale`) 400.0)
      (bind _output_get (set `self.Bounds Scale` (+ (`self.Bounds Scale`) 0.5)))
      (`MaterialInstanceDynamic.SetScalarParameterValue` (`self.DynamicMaterial`) "Bounds Scale" _output_get)
      (else
        (`/Engine/EditorBlueprintResources/StandardMacros.DoOnce` false
          (:`Completed`
            (`self.K2_DestroyActor`)))))))

(fn `UserConstructionScript`)