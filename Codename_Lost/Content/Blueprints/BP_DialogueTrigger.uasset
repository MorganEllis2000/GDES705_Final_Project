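; BP_DialogueTrigger is a one-shot trigger actor that plays a configurable sound, presumably a dialogue line, when a CharacterController actor overlaps it.
; The sound plays at the player character's location.
; If TurnOffLight is set, it also calls FlashlightOff on the player's CharacterController before destroying itself; otherwise it destroys itself right after starting the sound.
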(event `self.ReceiveActorBeginOverlap`
  (params (OtherActor :type "Actor Object Reference"))
  (bind _ascharacter_controller (cast `CharacterController` OtherActor))
  (`/Engine/EditorBlueprintResources/StandardMacros.IsValid` _ascharacter_controller
    (:`Is Valid`
      (`GameplayStatics.PlaySoundAtLocation` (`self.SoundToPlay`) (`self.K2_GetActorLocation` (`GameplayStatics.GetPlayerCharacter` 0)) (struct) 1.0 1.0 0.0 null null null null)
      (if (`self.TurnOffLight`)
        (bind _ascharacter_controller_2 (cast `CharacterController` (`GameplayStatics.GetPlayerCharacter` 0)))
        (`CharacterController.FlashlightOff` _ascharacter_controller_2)
        (`self.K2_DestroyActor`)
        (else
          (`self.K2_DestroyActor`))))))

(fn `UserConstructionScript`)