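; BP_Shadow is an AI-driven shadow enemy that plays an attached whispering sound and exchanges combat state with its Blackboard.
; Tick syncs attack flags while alive and watches Health; at zero it stops movement, flags death, detaches its controller, then destroys itself after a delay.
; Damage sets a Blackboard flag.
; ChangeVignette, not called here, adjusts post-process vignette from player distance, with a zero-alpha Lerp that yields no smoothing.
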(event `self.ReceiveBeginPlay`
  (bind _returnvalue (`GameplayStatics.SpawnSoundAttached` (`self.ShadowWisperingSoundCue`) (`self.RootComponent`) "None" (0.0 0.0 0.0) (struct) "KeepRelativeOffset" false 1.0 1.0 0.0 null null))
  (bind _ascharacter_controller (cast `CharacterController` (`GameplayStatics.GetPlayerCharacter` 0)))
  (set `self.Player` _ascharacter_controller))

(event `self.ReceiveTick`
  (params (DeltaSeconds :type "Float (single-precision)"))
  (`|ExecutionSequence`
    (:`then_0`
      (if (not (`self.IsDying`))
        (set `self.IsAttacking` (`BlackboardComponent.GetValueAsBool` (`AIBlueprintHelperLibrary.GetBlackboard` self) (`self.keyName`)))
        (bind _output_get (set `self.keyName` "CanAttack"))
        (`BlackboardComponent.SetValueAsBool` (`AIBlueprintHelperLibrary.GetBlackboard` self) _output_get (`self.CanAttack`))))
    (:`then_1`
      (if (<= (`HealthComponent.CurrentHealth` (`self.Health`)) 0.0)
        (`/Engine/EditorBlueprintResources/StandardMacros.DoOnce` false
          (:`Completed`
            (set `CharacterMovementComponent.MaxWalkSpeed` 0.0 (`self.CharacterMovement`))
            (`BlackboardComponent.SetValueAsBool` (`AIBlueprintHelperLibrary.GetBlackboard` self) (`self.IsDead`) true)
            (set `self.IsDying` true)
            (`self.DetachFromControllerPendingDestroy` self)
            (`KismetSystemLibrary.Delay` 3.4)
            (`AudioComponent.Stop` (stale `self.ReceiveBeginPlay` _returnvalue))
            (`self.K2_DestroyActor`)))))))

(event `self.ReceiveAnyDamage`
  (params (Damage :type "Float (single-precision)") (DamageType :type "DamageType Object Reference") (InstigatedBy :type "Controller Object Reference") (DamageCauser :type "Actor Object Reference"))
  (bind _output_get (set `self.keyName` "WasDamaged"))
  (`BlackboardComponent.SetValueAsBool` (`AIBlueprintHelperLibrary.GetBlackboard` (`AIBlueprintHelperLibrary.GetAIController` self)) _output_get true))

(fn `ChangeVignette`
  (bind _returnvalue (`BlackboardComponent.GetValueAsFloat` (`AIBlueprintHelperLibrary.GetBlackboard` (`AIBlueprintHelperLibrary.GetAIController` self)) (stale _output_get)))
  (if (> _returnvalue 600.0)
    (set `PostProcessComponent.Settings` (make `PostProcessSettings` :`VignetteIntensity` 1.0) (`self.PostProcess`))
    (else
      (bind _output_get (set `self.keyName` "DistFromPlayer"))
      (bind _returnvalue_2 (`KismetMathLibrary.Lerp` (- 3.0 (`KismetMathLibrary.NormalizeToRange` _returnvalue 1.0 300.0)) (`self.OldVignetteValue`)))
      (set `self.OldVignetteValue` _returnvalue_2)
      (set `PostProcessComponent.Settings` (make `PostProcessSettings` :`VignetteIntensity` _returnvalue_2) (`self.PostProcess`)))))

(fn `UserConstructionScript`)